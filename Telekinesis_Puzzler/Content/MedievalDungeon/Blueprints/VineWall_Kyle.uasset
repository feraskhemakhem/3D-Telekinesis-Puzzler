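; VineWall_Kyle is a vine wall actor that burns away when touched by an actor carrying a configured tag, intended for fire.
; The first tagged overlap calls BurnWall and sets a Lit flag so ignition happens only once.
; BurnWall loops to attach scaled pit-fire emitters to Wall2 at slightly stepped Y offsets, then destroys the actor after a short delay.
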(event Custom|BurnWall
  (for _index (range 0 10)
    (Effects|SpawnEmitterAttached "/Game/MedievalDungeon/Particles/P_Pit_Fire.P_Pit_Fire" (Variables|Default|GetWall2) "None" (Math|Vector|MakeVector 0.0 (Math|Conversions|ToFloat(Integer) _index) 5e+01) "0, 0, 0" "10.000000,5.000000,10.000000" "SnapToTarget")
    (Utilities|FlowControl|Delay 3.0)
    (Actor|DestroyActor)))

(event Collision|EventActorBeginOverlap
  (params (OtherActor :type Actor%20Object%20Reference))
  ;[1 1 1] Burn When Contacted By Fire
  (if (Actor|ActorHasTag OtherActor (Variables|Default|GetTagName))
    (if (not (Variables|Default|GetLit))
      (CallFunction|BurnWall)
      (Variables|Default|SetLit true))))

(fn ConstructionScript)