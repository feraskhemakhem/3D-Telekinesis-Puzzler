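; BP_DoorTorch is a torch that opens a crypt doorway when set alight.
; On BeginPlay it starts or ends its fire particle trails based on Lit, tags itself if lit, and caches the first BP_Crypt_Doorway tagged FireTrigger, assuming only one exists.
; When hit by an actor carrying the fire tag while unlit, it starts the trails, takes on that tag, becomes lit and calls OpenDoors on the door.
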(event EventBeginPlay
  ;[1 1 1] On Spawn, Start Trail If Lit, Then Find Door
  (Utilities|FlowControl|Sequence
    (:then_0
      (if (Variables|Default|GetLit)
        (Effects|Particles|Trails|BeginTrails (Variables|Default|GetP_Torch_Fire) "None" "None" "ETrailWidthMode_FromCentre" 0.0)
        (Variables|Default|SetTags (Utilities|Array|MakeArray (Variables|Default|GetTagName)))
        (else
          (Effects|Particles|Trails|EndTrails (Variables|Default|GetP_Torch_Fire)))))
    (:then_1
      (bind _outactors (Actor|GetAllActorsOfClasswithTag "/Game/MedievalDungeon/Blueprints/BP_Crypt_Doorway.BP_Crypt_Doorway_C" "FireTrigger"))
      (bind _asbp_crypt_doorway (Utilities|Casting|CastToBP_Crypt_Doorway (Utilities|Array|Get(acopy) _outactors))
        (:then
          (Variables|Default|SetDoor _asbp_crypt_doorway))
        (:CastFailed
          (Development|PrintString "Failed to Cast Door (DoorTorch)"))))))

(event Collision|EventHit
  (params (MyComp :type Primitive%20Component%20Object%20Reference) (Other :type Actor%20Object%20Reference) (OtherComp :type Primitive%20Component%20Object%20Reference) (bSelfMoved :type Boolean) (HitLocation :type Vector :default "0, 0, 0") (HitNormal :type Vector :default "0, 0, 0") (NormalImpulse :type Vector :default "0, 0, 0") (Hit :type Hit%20Result%20Structure%20%28by%20ref%29))
  ;[1 1 1] If Contacted by Fire and Not Lit, Light and Open Door
  (if (not (Variables|Default|GetLit)) ; If false, check tag
    (if (Actor|ActorHasTag Other (Variables|Default|GetTagName)) ; If true, make me burn
      (Effects|Particles|Trails|BeginTrails (Variables|Default|GetP_Torch_Fire) "None" "None" "ETrailWidthMode_FromCentre" 0.0)
      (Variables|Default|SetTags (Utilities|Array|MakeArray (Variables|Default|GetTagName)))
      (Variables|Default|SetLit true)
      (Default|OpenDoors (Variables|Default|GetDoor)))))

(fn ConstructionScript)