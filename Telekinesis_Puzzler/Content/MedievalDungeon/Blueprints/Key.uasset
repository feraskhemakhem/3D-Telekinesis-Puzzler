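; Key actor that opens a crypt doorway when it collides with a tagged actor.
; On BeginPlay it finds the first BP_Crypt_Doorway tagged "KeyTrigger" and caches it, printing a message if the cast fails.
; On Hit, if the other actor carries the TagName tag, it calls OpenDoors on the cached door and destroys itself.
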(event Collision|EventHit
  (params (MyComp :type Primitive%20Component%20Object%20Reference) (Other :type Actor%20Object%20Reference) (OtherComp :type Primitive%20Component%20Object%20Reference) (bSelfMoved :type Boolean) (HitLocation :type Vector :default "0, 0, 0") (HitNormal :type Vector :default "0, 0, 0") (NormalImpulse :type Vector :default "0, 0, 0") (Hit :type Hit%20Result%20Structure%20%28by%20ref%29))
  ;[1 1 1] If Placed In Door, Open Door
  (if (Actor|ActorHasTag Other (Variables|Default|GetTagName)) ; If true, Open door
    (Default|OpenDoors (Variables|Default|GetDoor))
    (Actor|DestroyActor)))

(event EventBeginPlay
  ;[1 1 1] Initialize Door Reference
  (bind _outactors (Actor|GetAllActorsOfClasswithTag "/Game/MedievalDungeon/Blueprints/BP_Crypt_Doorway.BP_Crypt_Doorway_C" "KeyTrigger"))
  (bind _asbp_crypt_doorway (Utilities|Casting|CastToBP_Crypt_Doorway (Utilities|Array|Get(acopy) _outactors))
    (:then
      (Variables|Default|SetDoor _asbp_crypt_doorway))
    (:CastFailed
      (Development|PrintString "Failed to Cast Door (Key)"))))

(fn ConstructionScript)