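; BP_Torch is a dungeon torch that starts lit or unlit and catches fire when hit by a burning actor.
; On BeginPlay, the Lit flag either starts the PTorchFire particle trails and sets the fire tag, or ends the trails.
; On Hit, an unlit torch checks the other actor for that tag, then ignites and takes the tag itself, so fire can spread.
; An already lit torch only prints a debug string.
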(event EventBeginPlay
  ;[1 1 1] On Spawn, Start Trail If Lit
  (if (Variables|Default|GetLit)
    (Effects|Particles|Trails|BeginTrails (Variables|Default|GetP_Torch_Fire) "None" "None" "ETrailWidthMode_FromCentre" 0.0)
    (Variables|Default|SetTags (Utilities|Array|MakeArray (Variables|Default|GetTagName)))
    (else
      (Effects|Particles|Trails|EndTrails (Variables|Default|GetP_Torch_Fire)))))

(event Collision|EventHit
  (params (MyComp :type Primitive%20Component%20Object%20Reference) (Other :type Actor%20Object%20Reference) (OtherComp :type Primitive%20Component%20Object%20Reference) (bSelfMoved :type Boolean) (HitLocation :type Vector :default "0, 0, 0") (HitNormal :type Vector :default "0, 0, 0") (NormalImpulse :type Vector :default "0, 0, 0") (Hit :type Hit%20Result%20Structure%20%28by%20ref%29))
  ;[1 1 1] If Contacted by Fire and Not Lit, Light
  (if (Variables|Default|GetLit) ; If false, check tag
    (Development|PrintString "Hello")
    (elif (Actor|ActorHasTag Other (Variables|Default|GetTagName)) ; If true, make me burn
      (Effects|Particles|Trails|BeginTrails (Variables|Default|GetP_Torch_Fire) "None" "None" "ETrailWidthMode_FromCentre" 0.0)
      (Variables|Default|SetTags (Utilities|Array|MakeArray (Variables|Default|GetTagName)))
      (Variables|Default|SetLit true))))

(fn ConstructionScript)