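; SpherePickup is a key pickup that opens a crypt doorway when it is placed in it.
; On BeginPlay it finds the first BP_Crypt_Doorway tagged KeyTrigger and caches it as the Door, printing debug messages.
; When it overlaps any actor with that same tag, it calls OpenDoors on the cached door and destroys itself.
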(event Collision|EventActorBeginOverlap
  (params (OtherActor :type Actor%20Object%20Reference))
  ;[1 1 1] If Placed In Door, Open Door
  (if (Actor|ActorHasTag OtherActor (Variables|Default|GetKeyTrigger)) ; If true, Open door
    (Default|OpenDoors (Variables|Default|GetDoor))
    (Actor|DestroyActor)))

(event EventBeginPlay
  ;[1 1 1] Initialize Door Reference
  (bind _outactors (Actor|GetAllActorsOfClasswithTag "/Game/MedievalDungeon/Blueprints/BP_Crypt_Doorway.BP_Crypt_Doorway_C" (Variables|Default|GetKeyTrigger)))
  (Development|PrintString (Utilities|GetDisplayName (Utilities|Array|Get(acopy) _outactors)))
  (bind _asbp_crypt_doorway (Utilities|Casting|CastToBP_Crypt_Doorway (Utilities|Array|Get(acopy) _outactors))
    (:then
      (Variables|Default|SetDoor _asbp_crypt_doorway))
    (:CastFailed
      (Development|PrintString "Failed to Cast Door (Key)"))))

(fn ConstructionScript
  (|CallParentFunction))